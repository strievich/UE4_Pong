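; BP_PongGameMode is the game mode for a two-player Pong match, controlling when play starts and where players spawn.
; ReadyToStartMatch holds the match until exactly two players are present.
; ChoosePlayerStart builds a tag from "P" and the current player count plus one, then returns the PlayerStart whose tag matches.
; The event graph and construction script are empty.
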(event EventBeginPlay)

(event EventTick
  (params (DeltaSeconds :type Float%20%28single-precision%29)))

(fn ConstructionScript)

(fn ReadytoStartMatch
  (return (== (Variables|Default|GetNumPlayers) 2)))

(fn ChoosePlayerStart
  (params (Player :type Controller%20Object%20Reference))
  (bind _asbp_pong_game_mode (Utilities|Casting|CastToBP_PongGameMode (Game|GetGameMode)))
  (bind _returnvalue (Class|PongGameMode|GetPlayersCount _asbp_pong_game_mode))
  (bind _outactors (Actor|GetAllActorsOfClass "/Script/Engine.PlayerStart"))
  (bind _array_element (Utilities|Array|ForEachLoopwithBreak _outactors)
    (:LoopBody
      (if (Utilities|Enum|Equal(Enum) (Utilities|String|BuildString(Integer) "" "P" (+ _returnvalue 1)) (Utilities|String|ToString(Name) (Variables|/Script/Engine.PlayerStart|GetPlayerStartTag _array_element)))
        (return _array_element)))))