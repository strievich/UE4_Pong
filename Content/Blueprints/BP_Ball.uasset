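; BP_Ball is the ball in a paddle-and-goal game, providing audio and camera feedback for its impacts.
; On BeginPlay it binds handlers to its goal, paddle and wall hit delegates, each playing its own sound at the ball's location.
; Paddle hits also trigger a horizontal world camera shake centered on the ball, while wall hits trigger a vertical one with the epicenter left unset.
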(event Custom|PlayGoalHitSound
  (Audio|PlaySoundatLocation "/Game/Audio/Goal.Goal" (Transformation|GetActorLocation) "0, 0, 0" 1.0 1.0 0.0 0 0 0))

(event Custom|CustomEvent_0
  (bind _returnvalue (Transformation|GetActorLocation))
  (Audio|PlaySoundatLocation "/Game/Audio/PaddleHit.PaddleHit" _returnvalue "0, 0, 0" 1.0 1.0 0.0 0 0 0)
  (Camera|PlayWorldCameraShake "/Game/Blueprints/CameraShakeHorisontal.CameraShakeHorisontal_C" _returnvalue 0.0 1e+05))

(event Custom|CustomEvent_1
  (Audio|PlaySoundatLocation "/Game/Audio/Wall_hit.Wall_hit" (Transformation|GetActorLocation) "0, 0, 0" 1.0 1.0 0.0 0 0 0)
  (Camera|PlayWorldCameraShake "/Game/Blueprints/CameraShakeVertical.CameraShakeVertical_C" "0, 0, 0" 0.0 1e+05))

(event EventBeginPlay
  (EventDispatchers|BindEventtoOnBallHitGoalDelegate (delegate Custom|PlayGoalHitSound))
  (EventDispatchers|BindEventtoOnBallHitPaddleDelegate (delegate Custom|CustomEvent_0))
  (EventDispatchers|BindEventtoOnBallHitWallDelegate (delegate Custom|CustomEvent_1)))

(event Collision|EventActorBeginOverlap
  (params (OtherActor :type Actor%20Object%20Reference)))

(event EventTick
  (params (DeltaSeconds :type Float%20%28single-precision%29)))

(fn ConstructionScript)